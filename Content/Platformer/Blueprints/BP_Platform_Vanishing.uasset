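; Platformer platform that vanishes after the player stands on it for a set lifetime, then reappears at its starting transform.
; A trigger zone flags the player pawn's presence, and Tick accumulates time while flagged, zeroing it otherwise.
; Reaching the lifetime hides the actor and disables its collision, then a delay precedes ReturnToStart, which restores transform, visibility and collision.
; Debug prints report overlaps and the timer.
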(event `self.ReceiveBeginPlay`
  ; Set Start Postion, Rotation & Scale
  (set `self.StartTransform` (`self.GetTransform`)))

(event `self.PlatformTriggerZone.OnComponentBeginOverlap`
  (params (OverlappedComponent :type "PrimitiveComponent Object Reference") (OtherActor :type "Actor Object Reference") (OtherComp :type "PrimitiveComponent Object Reference") (OtherBodyIndex :type Integer) (bFromSweep :type Boolean) (SweepResult :type "HitResult Structure (by ref)"))
  ; Collision Check
  (if (== OtherActor (`GameplayStatics.GetPlayerPawn` 0))
    (`|ExecutionSequence`
      (:`then_0`
        (`KismetSystemLibrary.PrintString` "Player is on the platform"))
      (:`then_1`
        (set `self.IsPlayerOnPlatform` true)))))

(event `self.PlatformTriggerZone.OnComponentEndOverlap`
  (params (OverlappedComponent :type "PrimitiveComponent Object Reference") (OtherActor :type "Actor Object Reference") (OtherComp :type "PrimitiveComponent Object Reference") (OtherBodyIndex :type Integer))
  ; Collision Check
  (if (== OtherActor (`GameplayStatics.GetPlayerPawn` 0))
    (`|ExecutionSequence`
      (:`then_0`
        (`KismetSystemLibrary.PrintString` "Player is off the platform"))
      (:`then_1`
        (set `self.IsPlayerOnPlatform` false)))))

(event `self.ReceiveTick`
  (params (DeltaSeconds :type "Float (single-precision)"))
  ; Set Timer For Platform
  (if (`self.IsPlayerOnPlatform`)
    (bind _output_get (set `self.TimeOnPlatform` (+ (`self.TimeOnPlatform`) DeltaSeconds)))
    (`|ExecutionSequence`
      (:`then_0`
        ; Checks if timer has reached the platform life time
        (if (>= (`self.TimeOnPlatform`) (`self.PlatformLifetime`))
          ; Hide & Disable Platform
          (`self.SetActorHiddenInGame` true)
          (`self.SetActorEnableCollision` false)
          (`KismetSystemLibrary.Delay` (`self.TimeInvisible`))
          (`self.ReturnToStart`)))
      (:`then_1`
        (`KismetSystemLibrary.PrintString` (`KismetStringLibrary.Conv_DoubleToString` _output_get))))
    (else
      (set `self.TimeOnPlatform` 0.0))))

(event `ReturnToStart`
  ; Reset Platform
  (`SceneComponent.K2_SetWorldTransform` (`self.DefaultSceneRoot`) (`self.StartTransform`) false true)
  (set `self.TimeOnPlatform` 0.0)
  (`self.SetActorHiddenInGame` false)
  (`self.SetActorEnableCollision` true))

(fn `UserConstructionScript`)