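; BP_NPC1 is a platformer NPC that shows an interaction prompt and plays timed dialog lines for the player.
; Its trigger zone toggles the prompt widget as the player, cached on BeginPlay, enters and leaves.
; ResetDialog restarts at the first line, then UpdateDialog writes each line to the player's CurrentDialogText, re-calling itself after a fixed delay and clearing the text at the end.
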(event `self.ReceiveBeginPlay`
  ; Creates the Player Reference
  (bind _asbp_third_person_character (cast `/Game/Platformer/Blueprints/BP_ThirdPersonCharacter` (`GameplayStatics.GetPlayerPawn` 0)))
  (set `self.PlayerReference` _asbp_third_person_character))

(event `self.NPCTriggerZone.OnComponentBeginOverlap`
  (params (OverlappedComponent :type "PrimitiveComponent Object Reference") (OtherActor :type "Actor Object Reference") (OtherComp :type "PrimitiveComponent Object Reference") (OtherBodyIndex :type Integer) (bFromSweep :type Boolean) (SweepResult :type "HitResult Structure (by ref)"))
  ; Checkng Overlap
  (if (== OtherActor (`self.PlayerReference`))
    (`SceneComponent.SetVisibility` (`self.Widget_InteractionPrompt`) true false)))

(event `self.NPCTriggerZone.OnComponentEndOverlap`
  (params (OverlappedComponent :type "PrimitiveComponent Object Reference") (OtherActor :type "Actor Object Reference") (OtherComp :type "PrimitiveComponent Object Reference") (OtherBodyIndex :type Integer))
  ; Checkng Overlap
  (if (== OtherActor (`self.PlayerReference`))
    (`SceneComponent.SetVisibility` (`self.Widget_InteractionPrompt`) false false)))

(event `UpdateDialog`
  ; Update Dialog
  (set `/Game/Platformer/Blueprints/BP_ThirdPersonCharacter.CurrentDialogText` (`|GetArrayItem` (`self.DialogLines`) (`self.CurrentDialogLine`)) (`self.PlayerReference`))
  (set `self.CurrentDialogLine` (+ (`self.CurrentDialogLine`) 1))
  (`KismetSystemLibrary.Delay` 2.0)
  (if (!= (`self.CurrentDialogLine`) (`KismetArrayLibrary.Array_Length` (`self.DialogLines`)))
    (`self.UpdateDialog`)
    (else
      (set `/Game/Platformer/Blueprints/BP_ThirdPersonCharacter.CurrentDialogText` "" (`self.PlayerReference`)))))

(event `ResetDialog`
  ; Reset Dialog
  (set `self.CurrentDialogLine` 0)
  (`self.UpdateDialog`))

(fn `UserConstructionScript`)